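; Interactable laptop actor that moves the player into a viewing position in front of it and shows its widget.
; Each Interact call flip-flops between entering and leaving, toggling player collision and widget visibility.
; Entering caches the pawn's transform, then the CamToLaptop timeline eases the pawn itself to CamPoint's location and Arrow's rotation.
; Leaving reverses that timeline to return the pawn to its cached transform.
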(event EventBeginPlay)

(event Collision|EventActorBeginOverlap
  (params (OtherActor :type Actor%20Object%20Reference)))

(event EventTick
  (params (DeltaSeconds :type Float%20%28single-precision%29)))

(event EventInteract
  (bind _returnvalue (Game|Player|GetPlayerPawn 0))
  (bind _returnvalue_2 (Game|GetPlayerController 0))
  (bind _returnvalue_3 (Pawn|GetControlledPawn _returnvalue_2))
  ;[1 1 1] interact
  (Utilities|FlowControl|FlipFlop
    (:A
      (Collision|SetActorEnableCollision _returnvalue false)
      (Rendering|SetVisibility (Variables|Default|GetWidget) true false)
      (Variables|Default|SetPlayer%20init%20loc (Transformation|GetActorLocation _returnvalue))
      (Variables|Default|SetPlayer%20init%20rot (Transformation|GetActorRotation _returnvalue))
      (Variables|Default|SetPlayer%20target%20rot (Transformation|GetWorldRotation (Variables|Default|GetArrow)))
      (Variables|Default|SetPlayer%20target%20loc (Transformation|GetWorldLocation (Variables|Default|GetCamPoint)))
      (bind _progress (Timeline|Cam%20to%20Laptop Play)
        (:Update
          (Transformation|SetActorLocation _returnvalue_3 (Math|Interpolation|Ease "EaseOut" _progress (Variables|Default|GetPlayer%20init%20loc) (Variables|Default|GetPlayer%20target%20loc) 2.0) false false)
          (Transformation|SetActorRotation _returnvalue_3 (Math|Interpolation|Ease "EaseOut" _progress (Variables|Default|GetPlayer%20init%20rot) (Variables|Default|GetPlayer%20target%20rot) true)))))
    (:B
      (Collision|SetActorEnableCollision (Game|Player|GetPlayerPawn 0) true)
      (Rendering|SetVisibility (Variables|Default|GetWidget) false false)
      (Timeline|Cam%20to%20Laptop Reverse))))

(fn ConstructionScript)