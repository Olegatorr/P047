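; Blueprint function library with a shared check for whether the player is looking at something interactable.
; CanInteract line-traces on the Visibility channel from the player camera along its forward vector over a short fixed reach.
; A hit within that reach whose actor implements the Interaction interface returns true with that actor and the hit distance.
; Any other result returns false with the distance.
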(fn CanInteract?
  (bind _returnvalue (Game|GetPlayerCharacter 0))
  (bind _returnvalue_2 (Game|GetPlayerCameraManager _returnvalue))
  (bind _returnvalue_3 (Camera|GetCameraLocation _returnvalue_2))
  (bind (_outhit _returnvalue_4) (Collision|LineTraceByChannel 0 _returnvalue_3 (+ (* (Math|Vector|GetForwardVector (Camera|GetCameraRotation _returnvalue_2)) 2e+02) _returnvalue_3) "TraceTypeQuery1" false 0 "None" false))
  (if _returnvalue_4
    (Math|Float|CompareFloat (.distance _outhit) 2e+02
      (:>
        _)
      (:==
        (if (Utilities|DoesObjectImplementInterface (.hitactor _outhit) "/Game/Blueprints/Interaction.Interaction_C") :!label _label
          (return true (.hitactor _outhit) (.distance _outhit))
          (else
            _)))
      (:<
        (goto _label))))
  (return false 0 (.distance _outhit)))