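; Lamp actor Blueprint with an IsBroken flag that turns it into a randomly flickering broken light.
; When broken, the construction script darkens the lamp material, hides the RectLight and adds a hidden movable point light; otherwise it applies the lit material.
; On BeginPlay, a broken lamp loops through short random delays and a FlipFlop, toggling the material and point light together.
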(event EventBeginPlay
  (bind _lamp (Variables|Default|Getlamp))
  (bind _spawned_point_light (Variables|Default|GetSpawned%20Point%20Light))
  (if (Variables|Default|GetIs%20broken?)
    (Utilities|FlowControl|Delay (Math|Random|RandomFloatinRange 0.01 0.6) :!label _label)
    (Utilities|FlowControl|FlipFlop
      (:A
        (Rendering|Material|SetMaterial _lamp 0 "/Game/L0/Materials/darkgrey.darkgrey")
        (Rendering|SetVisibility _spawned_point_light false false)
        (goto _label))
      (:B
        (Rendering|Material|SetMaterial _lamp 0 "/Game/L0/Materials/lampmat.lampmat")
        (Rendering|SetVisibility _spawned_point_light true false)
        (goto _label)))))

(event Collision|EventActorBeginOverlap
  (params (OtherActor :type Actor%20Object%20Reference)))

(event EventTick
  (params (DeltaSeconds :type Float%20%28single-precision%29)))

(fn ConstructionScript
  (bind _lamp (Variables|Default|Getlamp))
  (if (Variables|Default|GetIs%20broken?)
    (Rendering|Material|SetMaterial _lamp 0 "/Game/L0/Materials/darkgrey.darkgrey")
    (bind _returnvalue (AddComponent|AddPointLightComponent false))
    (bind _output_get (Variables|Default|SetSpawned%20Point%20Light _returnvalue))
    (Transformation|SetMobility _output_get "Movable")
    (Rendering|Components|Light|SetIntensity _output_get 2e+02)
    (Rendering|Lighting|SetAttenuationRadius _output_get 5e+02)
    (Rendering|SetVisibility _output_get false false)
    (Rendering|SetVisibility (Variables|Default|GetRectLight) false false)
    (else
      (Rendering|Material|SetMaterial _lamp 0 "/Game/L0/Materials/lampmat.lampmat"))))